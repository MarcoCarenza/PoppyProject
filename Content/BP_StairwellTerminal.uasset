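; BP_StairwellTerminal is an interactable terminal that shows focus and highlight feedback on its mesh.
; Focus changes set FacingTerminal on the player's BP_HorrorCharacter, clear TerminalViewing and toggle the mesh's custom depth rendering.
; HighlightItem briefly enables custom depth with a stencil value, then switches it off after a delay.
; It exposes its interaction widget through a getter, while skillcheck and overlay-material nodes remain unconnected.
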(event `self.Interface_ToggleFocus`
  (params (Focus :type Boolean))
  (bind _asbp_horror_character (cast `/Game/Variant_Horror/Blueprints/BP_HorrorCharacter` (`GameplayStatics.GetPlayerCharacter` 0)))
  (set `/Game/Variant_Horror/Blueprints/BP_HorrorCharacter.FacingTerminal?` Focus _asbp_horror_character)
  (set `/Game/Variant_Horror/Blueprints/BP_HorrorCharacter.TerminalViewing` null _asbp_horror_character)
  (`PrimitiveComponent.SetRenderCustomDepth` (`self.TerminalMesh`) Focus))

(event `self.ReceiveBeginPlay`
  (`PrimitiveComponent.SetRenderCustomDepth` (`self.TerminalMesh`) false))

(event `HighlightItem`
  (bind _terminalmesh (`self.TerminalMesh`))
  (`PrimitiveComponent.SetRenderCustomDepth` (`self.TerminalMesh`) true)
  (`PrimitiveComponent.SetCustomDepthStencilValue` _terminalmesh 5)
  (`KismetSystemLibrary.Delay` 2.0)
  (`PrimitiveComponent.SetRenderCustomDepth` _terminalmesh false))

(event `self.ReceiveActorBeginOverlap`
  (params (OtherActor :type "Actor Object Reference")))

(fn `GetInteractionWidgetRef`
  (returns (Ref :type "WidgetComponent Object Reference"))
  (return (`self.Widget`)))

(fn `UserConstructionScript`)