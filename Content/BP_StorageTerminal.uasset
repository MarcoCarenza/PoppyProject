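; BP_StorageTerminal is an interactable terminal that highlights its mesh and shows a key-spam prompt when the player is near.
; Interface focus toggles custom depth on the mesh and updates the horror character's terminal-facing state, while HighlightItem shows a two-second stencil highlight.
; Entering the box spawns a WBP_SpamE widget with the required press count, and leaving removes it.
; Press-counting and overlay-material logic remain in the graph but are unconnected.
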(event `self.Interface_ToggleFocus`
  (params (Focus :type Boolean))
  (bind _asbp_horror_character (cast `/Game/Variant_Horror/Blueprints/BP_HorrorCharacter` (`GameplayStatics.GetPlayerCharacter` 0)))
  (set `/Game/Variant_Horror/Blueprints/BP_HorrorCharacter.FacingTerminal?` Focus _asbp_horror_character)
  (set `/Game/Variant_Horror/Blueprints/BP_HorrorCharacter.TerminalViewing` null _asbp_horror_character)
  (`PrimitiveComponent.SetRenderCustomDepth` (`self.TerminalMesh`) Focus))

(event `self.ReceiveBeginPlay`
  (`PrimitiveComponent.SetRenderCustomDepth` (`self.TerminalMesh`) false))

(event `HighlightItem`
  (bind _terminalmesh (`self.TerminalMesh`))
  (`PrimitiveComponent.SetRenderCustomDepth` (`self.TerminalMesh`) true)
  (`PrimitiveComponent.SetCustomDepthStencilValue` _terminalmesh 5)
  (`KismetSystemLibrary.Delay` 2.0)
  (`PrimitiveComponent.SetRenderCustomDepth` _terminalmesh false))

(event `self.Box.OnComponentBeginOverlap`
  (params (OverlappedComponent :type "PrimitiveComponent Object Reference") (OtherActor :type "Actor Object Reference") (OtherComp :type "PrimitiveComponent Object Reference") (OtherBodyIndex :type Integer) (bFromSweep :type Boolean) (SweepResult :type "HitResult Structure (by ref)"))
  (bind _asbp_horror_character (cast `/Game/Variant_Horror/Blueprints/BP_HorrorCharacter` OtherActor))
  (`self.EnableInput` _asbp_horror_character (`GameplayStatics.GetPlayerController` 0))
  (bind _returnvalue (`|CreateWidget` "/Game/Variant_Horror/UI/WBP_SpamE.WBP_SpamE_C"))
  (bind _output_get (set `self.widgetRef` _returnvalue))
  (`UserWidget.AddToViewport` _output_get 0)
  (set `/Game/Variant_Horror/UI/WBP_SpamE.pressesNeeded` (`self.pressedNeeded`) _output_get))

(event `self.Box.OnComponentEndOverlap`
  (params (OverlappedComponent :type "PrimitiveComponent Object Reference") (OtherActor :type "Actor Object Reference") (OtherComp :type "PrimitiveComponent Object Reference") (OtherBodyIndex :type Integer))
  (cast `/Game/Variant_Horror/Blueprints/BP_HorrorCharacter` OtherActor)
  (`self.DisableInput` (`GameplayStatics.GetPlayerController` 0))
  (`Widget.RemoveFromParent` (stale `self.Box.OnComponentBeginOverlap` _returnvalue)))

(fn `GetInteractionWidgetRef`
  (returns (Ref :type "WidgetComponent Object Reference"))
  (return (`self.Widget`)))

(fn `UserConstructionScript`)