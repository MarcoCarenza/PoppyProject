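; BP_Servers is a server prop actor whose appearance follows the LightsOn state of the player's BP_HorrorCharacter.
; On BeginPlay and every Tick, it casts player character 0 and reads that flag.
; It then sets the first material slot of six static meshes to one of two sci-fi hard-surface materials, polling each frame rather than responding to an event.
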(event `self.ReceiveBeginPlay`
  (bind _staticmesh9 (`self.StaticMesh9`))
  (bind _asbp_horror_character (cast `/Game/Variant_Horror/Blueprints/BP_HorrorCharacter` (`GameplayStatics.GetPlayerCharacter` 0) :!label _label))
  (if (`/Game/Variant_Horror/Blueprints/BP_HorrorCharacter.LightsOn?` _asbp_horror_character)
    (`PrimitiveComponent.SetMaterial` _staticmesh9 0 "/Game/High_Tech_Base/Materials/MI_Sci_Fi_Hard_Surface_02.MI_Sci_Fi_Hard_Surface_02")
    (`PrimitiveComponent.SetMaterial` (`self.StaticMesh10`) 0 "/Game/High_Tech_Base/Materials/MI_Sci_Fi_Hard_Surface_02.MI_Sci_Fi_Hard_Surface_02")
    (`PrimitiveComponent.SetMaterial` (`self.StaticMesh1`) 0 "/Game/High_Tech_Base/Materials/MI_Sci_Fi_Hard_Surface_02.MI_Sci_Fi_Hard_Surface_02")
    (`PrimitiveComponent.SetMaterial` (`self.StaticMesh6`) 0 "/Game/High_Tech_Base/Materials/MI_Sci_Fi_Hard_Surface_02.MI_Sci_Fi_Hard_Surface_02")
    (`PrimitiveComponent.SetMaterial` (`self.StaticMesh2`) 0 "/Game/High_Tech_Base/Materials/MI_Sci_Fi_Hard_Surface_02.MI_Sci_Fi_Hard_Surface_02")
    (`PrimitiveComponent.SetMaterial` (`self.StaticMesh11`) 0 "/Game/High_Tech_Base/Materials/MI_Sci_Fi_Hard_Surface_02.MI_Sci_Fi_Hard_Surface_02")
    (else
      (`PrimitiveComponent.SetMaterial` _staticmesh9 0 "/Game/High_Tech_Base/Materials/MI_Sci_Fi_Hard_Surface_Server.MI_Sci_Fi_Hard_Surface_Server")
      (`PrimitiveComponent.SetMaterial` (`self.StaticMesh10`) 0 "/Game/High_Tech_Base/Materials/MI_Sci_Fi_Hard_Surface_Server.MI_Sci_Fi_Hard_Surface_Server")
      (`PrimitiveComponent.SetMaterial` (`self.StaticMesh1`) 0 "/Game/High_Tech_Base/Materials/MI_Sci_Fi_Hard_Surface_Server.MI_Sci_Fi_Hard_Surface_Server")
      (`PrimitiveComponent.SetMaterial` (`self.StaticMesh6`) 0 "/Game/High_Tech_Base/Materials/MI_Sci_Fi_Hard_Surface_Server.MI_Sci_Fi_Hard_Surface_Server")
      (`PrimitiveComponent.SetMaterial` (`self.StaticMesh2`) 0 "/Game/High_Tech_Base/Materials/MI_Sci_Fi_Hard_Surface_Server.MI_Sci_Fi_Hard_Surface_Server")
      (`PrimitiveComponent.SetMaterial` (`self.StaticMesh11`) 0 "/Game/High_Tech_Base/Materials/MI_Sci_Fi_Hard_Surface_Server.MI_Sci_Fi_Hard_Surface_Server"))))

(event `self.ReceiveTick`
  (params (DeltaSeconds :type "Float (single-precision)"))
  (goto _label))

(fn `UserConstructionScript`)