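; SoundVolume is an overlap-driven actor that makes an FMOD sound audible while BP_HorrorCharacter is inside it.
; On BeginPlay it starts SoundToPlay as a 2D event with its Volume parameter at zero, optionally enabling a Muffling parameter.
; Overlap begin and end switch Volume between full and zero on the running instance, so the event is never restarted or stopped here.
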(event `self.ReceiveBeginPlay`
  (bind _returnvalue (`FMODBlueprintStatics.PlayEvent2D` (`self.SoundToPlay`)))
  (bind _output_get (set `self.Instance` _returnvalue))
  (`FMODBlueprintStatics.EventInstanceSetParameter` _output_get "Volume" 0.0)
  (if (`self.Muffling`)
    (`FMODBlueprintStatics.EventInstanceSetParameter` (`self.Instance`) "Muffling" 1.0)))

(event `self.ReceiveActorBeginOverlap`
  (params (OtherActor :type "Actor Object Reference"))
  (cast `/Game/Variant_Horror/Blueprints/BP_HorrorCharacter` OtherActor)
  (`FMODBlueprintStatics.EventInstanceSetParameter` (`self.Instance`) "Volume" 1.0))

(event `self.ReceiveActorEndOverlap`
  (params (OtherActor :type "Actor Object Reference"))
  (cast `/Game/Variant_Horror/Blueprints/BP_HorrorCharacter` OtherActor)
  (`FMODBlueprintStatics.EventInstanceSetParameter` (`self.Instance`) "Volume" 0.0))

(fn `UserConstructionScript`)