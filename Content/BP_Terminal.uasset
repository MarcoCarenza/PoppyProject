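; BP_Terminal is an interactable computer terminal actor for the horror character to face and view.
; When focus toggles, it sets the player character's terminal state and toggles a custom-depth outline on its meshes.
; On begin play, an HQMonitor flag picks between the single terminal mesh and separate screen, base and keyboard parts.
; A highlight event flashes a stencil-tinted outline briefly, and the interaction widget is exposed through a getter.
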(event `/Game/Variant_Horror/Interaction/BI_Interaction.Interface_ToggleFocus`
  (params (Focus :type Boolean))
  (bind _asbp_horror_character (cast `/Game/Variant_Horror/Blueprints/BP_HorrorCharacter` (`GameplayStatics.GetPlayerCharacter` 0)))
  (set `/Game/Variant_Horror/Blueprints/BP_HorrorCharacter.FacingTerminal?` Focus _asbp_horror_character)
  (set `/Game/Variant_Horror/Blueprints/BP_HorrorCharacter.TerminalViewing` self _asbp_horror_character)
  (`PrimitiveComponent.SetRenderCustomDepth` (`self.TerminalMesh`) Focus)
  (`PrimitiveComponent.SetRenderCustomDepth` (`self.Screen`) Focus)
  (`PrimitiveComponent.SetRenderCustomDepth` (`self.Keyboard`) Focus))

(event `self.ReceiveBeginPlay`
  (bind _screen (`self.Screen`))
  (bind _screen_2 (`self.Screen`))
  (`PrimitiveComponent.SetRenderCustomDepth` (`self.TerminalMesh`) false)
  (`PrimitiveComponent.SetRenderCustomDepth` (`self.Screen`) false)
  (`PrimitiveComponent.SetRenderCustomDepth` (`self.Keyboard`) false)
  (if (`self.HQMonitor?`)
    (`SceneComponent.SetHiddenInGame` (`self.TerminalMesh`) true false)
    (`SceneComponent.SetVisibility` _screen true false)
    (`SceneComponent.SetVisibility` (`self.Base`) true false)
    (`SceneComponent.SetVisibility` (`self.Keyboard`) true false)
    (`SceneComponent.SetHiddenInGame` _screen false false)
    (`SceneComponent.SetHiddenInGame` (`self.Base`) false false)
    (`SceneComponent.SetHiddenInGame` (`self.Keyboard`) false false)
    (else
      (`SceneComponent.SetVisibility` _screen_2 false false)
      (`SceneComponent.SetVisibility` (`self.Base`) false false)
      (`SceneComponent.SetVisibility` (`self.Keyboard`) false false)
      (`SceneComponent.SetHiddenInGame` _screen_2 true false)
      (`SceneComponent.SetHiddenInGame` (`self.Base`) true false)
      (`SceneComponent.SetHiddenInGame` (`self.Keyboard`) true false)
      (`PrimitiveComponent.SetCollisionEnabled` _screen_2 "NoCollision")
      (`PrimitiveComponent.SetCollisionEnabled` (`self.Base`) "NoCollision")
      (`PrimitiveComponent.SetCollisionEnabled` (`self.Keyboard`) "NoCollision"))))

(event `HighlightItem`
  (bind _terminalmesh (`self.TerminalMesh`))
  (`PrimitiveComponent.SetRenderCustomDepth` (`self.TerminalMesh`) true)
  (`PrimitiveComponent.SetRenderCustomDepth` (`self.Screen`) true)
  (`PrimitiveComponent.SetRenderCustomDepth` (`self.Keyboard`) true)
  (`PrimitiveComponent.SetCustomDepthStencilValue` _terminalmesh 5)
  (`PrimitiveComponent.SetCustomDepthStencilValue` (`self.Keyboard`) 5)
  (`PrimitiveComponent.SetCustomDepthStencilValue` (`self.Screen`) 5)
  (`KismetSystemLibrary.Delay` 2.0)
  (`PrimitiveComponent.SetRenderCustomDepth` _terminalmesh false)
  (`PrimitiveComponent.SetRenderCustomDepth` (`self.Keyboard`) false)
  (`PrimitiveComponent.SetRenderCustomDepth` (`self.Screen`) false))

(event `self.Box.OnComponentBeginOverlap`
  (params (OverlappedComponent :type "PrimitiveComponent Object Reference") (OtherActor :type "Actor Object Reference") (OtherComp :type "PrimitiveComponent Object Reference") (OtherBodyIndex :type Integer) (bFromSweep :type Boolean) (SweepResult :type "HitResult Structure (by ref)")))

(event `self.Box.OnComponentEndOverlap`
  (params (OverlappedComponent :type "PrimitiveComponent Object Reference") (OtherActor :type "Actor Object Reference") (OtherComp :type "PrimitiveComponent Object Reference") (OtherBodyIndex :type Integer)))

(fn `GetInteractionWidgetRef`
  (returns (Ref :type "WidgetComponent Object Reference"))
  (return (`self.Widget`)))

(fn `UserConstructionScript`)