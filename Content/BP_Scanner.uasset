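; BP_Scanner is a scan pulse in a horror game that highlights terminals and draws noise attention.
; DoScan flags BP_HorrorCharacter as scanning, reports a loud noise event, and runs a timeline that scales the actor and animates material opacity.
; The sphere's query collision is enabled only during the pulse, calling HighlightItem on each overlapped BP_Terminal.
; When finished, it hides itself, clears the flag, and prints the player's distance to AI_Monster.
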(event `self.ReceiveBeginPlay`)

(event `self.PawnNoiseEmitter.OnComponentActivated`
  (params (Component :type "ActorComponent Object Reference") (bReset :type Boolean))
  (`PawnNoiseEmitterComponent.MakeNoise` (`self.PawnNoiseEmitter`) self 1.0 (`self.K2_GetActorLocation`)))

(event `DoScan`
  (bind _returnvalue_location (`KismetMathLibrary.BreakTransform` (`self.GetTransform` (`GameplayStatics.GetPlayerCharacter` 0))))
  (`self.SetActorHiddenInGame` false)
  (`PrimitiveComponent.SetCollisionEnabled` (`self.Sphere`) "QueryOnly")
  (`AISense_Hearing.ReportNoiseEvent` (`self.K2_GetActorLocation`) 2.0 null 5000.0)
  (`GameplayStatics.PlaySound2D` "/Game/Audio/Scanning.Scanning" 1.0 1.0 0.0 null null)
  (bind _returnvalue (`GameplayStatics.GetActorOfClass` "/Game/Variant_Horror/Blueprints/BP_HorrorCharacter.BP_HorrorCharacter_C"))
  (set `/Game/Variant_Horror/Blueprints/BP_HorrorCharacter.Scanning?` true _returnvalue)
  (bind (_direction _opacity2 _scannerexpandsize2) (`Timeline|ExpandScanner` :!via `PlayFromStart`)
    (:`Update`
      (`self.SetActorScale3D` (`KismetMathLibrary.Conv_DoubleToVector` _scannerexpandsize2))
      (`MeshComponent.SetScalarParameterValueOnMaterials` (`self.Sphere`) "Scan_Opacity" _opacity2))
    (:`Finished`
      (`PrimitiveComponent.SetCollisionEnabled` (`self.Sphere`) "NoCollision")
      (`self.SetActorScale3D` (0.0 0.0 0.0))
      (`self.SetActorHiddenInGame` true)
      (`GameplayStatics.PlaySound2D` "/Game/Audio/ScanComplete.ScanComplete" 3.0 1.0 0.0 null null)
      (bind _returnvalue_2 (`GameplayStatics.GetActorOfClass` "/Game/Variant_Horror/Blueprints/BP_HorrorCharacter.BP_HorrorCharacter_C"))
      (set `/Game/Variant_Horror/Blueprints/BP_HorrorCharacter.Scanning?` false _returnvalue_2)
      (bind _returnvalue_3 (`GameplayStatics.GetActorOfClass` "/Game/AI/AI_Monster.AI_Monster_C"))
      (bind _returnvalue_location_2 (`KismetMathLibrary.BreakTransform` (`self.GetTransform` _returnvalue_3)))
      (`KismetSystemLibrary.PrintString` (`KismetStringLibrary.Concat_StrStr` "Distance to monster is: " (`KismetStringLibrary.Conv_IntToString` (/ (`KismetMathLibrary.Round` (`KismetMathLibrary.Vector_Distance` _returnvalue_location _returnvalue_location_2)) 100)) "m")))))

(event `self.Sphere.OnComponentBeginOverlap`
  (params (OverlappedComponent :type "PrimitiveComponent Object Reference") (OtherActor :type "Actor Object Reference") (OtherComp :type "PrimitiveComponent Object Reference") (OtherBodyIndex :type Integer) (bFromSweep :type Boolean) (SweepResult :type "HitResult Structure (by ref)"))
  (bind _asbp_terminal (cast `/Game/BP_Terminal` OtherActor))
  (`/Game/BP_Terminal.HighlightItem` _asbp_terminal))

(fn `UserConstructionScript`)